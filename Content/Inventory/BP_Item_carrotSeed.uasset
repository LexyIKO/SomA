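; Carrot seed inventory item that plants carrots in a garden bed when used.
; On use, it casts the character's interacting actor to a garden bed and proceeds only if the character is in collision and nothing is planted there.
; It then removes itself from the character's inventory and tells the bed to handle the carrot seed interaction.
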(event `self.OnUse`
  (params (Character :type "AvatarCPP Object Reference"))
  (bind _asbp_garden_bed (cast `/Game/Locations/MainLocation/Interactive_Object/BP_GardenBed` (`AvatarCPP.InteractingActor` Character)))
  (if (and (`AvatarCPP.InCollision` Character) (not (`/Game/Locations/MainLocation/Interactive_Object/BP_GardenBed.IsSomethingPlanted` _asbp_garden_bed)))
    (`InventoryComponent.RemoveItem` (`AvatarCPP.Inventory` Character) self)
    (`/Game/Locations/MainLocation/Interactive_Object/BP_GardenBed.InteractWithCarrotSeed` _asbp_garden_bed)))
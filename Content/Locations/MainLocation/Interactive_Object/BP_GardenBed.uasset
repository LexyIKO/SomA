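; Garden bed interactive object where the player grows and harvests potatoes or carrots.
; Interact opens the inventory widget in UI-only input mode unless a crop is fully grown, in which case it adds that item to the avatar's inventory and clears the bed.
; Separate seed events plant an empty bed, swapping added static mesh components through three timed growth stages using Delays, then record the crop type for harvest.
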(event `self.Interact`
  (bind _returnvalue (`GameplayStatics.GetPlayerController` 0))
  (if (`self.FullyGrown`)
    (switch `int` (`self.WhichPlantIsFullyGrown`)
      (:`0`
        ;[1 1 1] Добавление картофеля если был посажен картофель и он дорос
        (bind _asavatar_cpp (cast `AvatarCPP` (`GameplayStatics.GetPlayerPawn` 0)))
        (bind _returnvalue_2 (`|GenericCreateObject` (`self.PotatoClassRef`) (`KismetSystemLibrary.GetOuterObject` _asavatar_cpp)))
        (`InventoryComponent.AddItem` (`AvatarCPP.Inventory` _asavatar_cpp) _returnvalue_2)
        (set `self.FullyGrown` false)
        (set `self.IsSomethingPlanted` false)
        (`ActorComponent.K2_DestroyComponent` (`self.LastPotatoStaticMesh`)))
      (:`1`
        ;[1 1 1] Добавление моркови если была посажена морковь и она доросла
        (bind _asavatar_cpp_2 (cast `AvatarCPP` (`GameplayStatics.GetPlayerPawn` 0)))
        (bind _returnvalue_3 (`|GenericCreateObject` (`self.CarrotClassRef`) (`KismetSystemLibrary.GetOuterObject` _asavatar_cpp_2)))
        (`InventoryComponent.AddItem` (`AvatarCPP.Inventory` _asavatar_cpp_2) _returnvalue_3)
        (set `self.FullyGrown` false)
        (set `self.IsSomethingPlanted` false)
        (`ActorComponent.K2_DestroyComponent` (`self.LastCarrotStaticMesh`))))
    (else
      ;[1 1 1] Открытие инвентаря
      (bind _returnvalue_4 (`|CreateWidget` "/Game/Inventory/WBP_Inventory.WBP_Inventory_C" (`GameplayStatics.GetPlayerController` 0)))
      (`UserWidget.AddToViewport` _returnvalue_4 0)
      (set `PlayerController.bShowMouseCursor` true _returnvalue)
      (`WidgetBlueprintLibrary.SetInputMode_UIOnlyEx` _returnvalue _returnvalue_4))))

(event `InteractWithPotatoSeed`
  ;[1 1 1] При взаимодействии с семенами картофеля
  (if (not (`self.IsSomethingPlanted`))
    (bind _returnvalue (`AddComponent|NODE_AddStaticMeshComponent-0` :`RelativeTransform` (`KismetMathLibrary.MakeTransform` (0.0 0.0 10.0) (struct :`Yaw` -90.0))))
    (set `self.IsSomethingPlanted` true)
    (`KismetSystemLibrary.Delay` 5.0)
    (`ActorComponent.K2_DestroyComponent` _returnvalue)
    (bind _returnvalue_2 (`AddComponent|NODE_AddStaticMeshComponent-1` :`RelativeTransform` (`KismetMathLibrary.MakeTransform` (0.0 0.0 20.0) (struct :`Yaw` -90.0))))
    (`KismetSystemLibrary.Delay` 5.0)
    (`ActorComponent.K2_DestroyComponent` _returnvalue_2)
    (bind _returnvalue_3 (`AddComponent|NODE_AddStaticMeshComponent-2` :`RelativeTransform` (`KismetMathLibrary.MakeTransform` (0.0 0.0 35.0) (struct :`Yaw` -90.0))))
    (set `self.FullyGrown` true)
    (set `self.LastPotatoStaticMesh` _returnvalue_3)
    (set `self.WhichPlantIsFullyGrown` 0)))

(event `InteractWithCarrotSeed`
  ;[1 1 1] При взаимодействии с семенами моркови
  (if (not (`self.IsSomethingPlanted`))
    (bind _returnvalue (`AddComponent|NODE_AddStaticMeshComponent-3` :`RelativeTransform` (`KismetMathLibrary.MakeTransform` (0.0 0.0 10.0))))
    (set `self.IsSomethingPlanted` true)
    (`KismetSystemLibrary.Delay` 5.0)
    (`ActorComponent.K2_DestroyComponent` _returnvalue)
    (bind _returnvalue_2 (`AddComponent|NODE_AddStaticMeshComponent-4` :`RelativeTransform` (`KismetMathLibrary.MakeTransform` (0.0 0.0 35.0))))
    (`KismetSystemLibrary.Delay` 5.0)
    (`ActorComponent.K2_DestroyComponent` _returnvalue_2)
    (bind _returnvalue_3 (`AddComponent|NODE_AddStaticMeshComponent-5` :`RelativeTransform` (`KismetMathLibrary.MakeTransform` (0.0 0.0 50.0))))
    (set `self.FullyGrown` true)
    (set `self.LastCarrotStaticMesh` _returnvalue_3)
    (set `self.WhichPlantIsFullyGrown` 1)))

(fn `UserConstructionScript`)